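; Heavy enemy Blueprint that wanders randomly while not alert.
; BeginPlay applies MoveSpeed to the movement component's max walk speed.
; Tick checks IsAlert on the owning MyAICharacter and, when false, uses a Delay to throttle AI Move To orders toward random navigable points within Radius of itself.
; A successful move only prints debug text after a delay, and this graph has no alert behavior.
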(event EventBeginPlay
  (Variables|/Script/Engine.CharacterMovementComponent|SetMaxWalkSpeed (Variables|Character|GetCharacterMovement) (Variables|Default|GetMoveSpeed)))

(event Collision|EventActorBeginOverlap
  (params (OtherActor :type Actor%20Object%20Reference)))

(event EventTick
  (params (DeltaSeconds :type Float%20%28single-precision%29))
  (bind _asmy_aicharacter (Utilities|Casting|CastToMyAICharacter (Class|PawnMovementComponent|GetPawnOwner (Variables|Character|GetCharacterMovement))))
  (if (not (Variables|/Script/MothGame.MyAICharacter|GetisAlert _asmy_aicharacter))
    (Utilities|FlowControl|Delay 3.0)
    (Utilities|Casting|CastToMyAICharacter (Class|PawnMovementComponent|GetPawnOwner (Variables|Character|GetCharacterMovement)))
    (AI|AIMoveTo 0 (.RandomLocation (Class|NavigationSystemV1|GetRandomPointinNavigableRadius (Transformation|GetActorLocation) (Variables|Default|GetRadius) 0 0)) 0 1e+02 false
      (:OnSuccess
        (Utilities|FlowControl|Delay 3.0)
        (Development|PrintText "Random")))))

(fn ConstructionScript)