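; Base enemy AI Blueprint that wanders around an origin point and speeds up when alerted.
; BeginPlay applies MoveSpeed to the movement component, and Tick casts the pawn to MyAICharacter to read IsAlert.
; When alert it raises walk speed without resetting it; otherwise Tick-driven Delays pace moves to random navigable points within Radius of VecOPos, followed by a debug print.
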(event EventBeginPlay
  (Variables|/Script/Engine.CharacterMovementComponent|SetMaxWalkSpeed (Variables|Character|GetCharacterMovement) (Variables|Default|GetMoveSpeed)))

(event Collision|EventActorBeginOverlap
  (params (OtherActor :type Actor%20Object%20Reference)))

(event EventTick
  (params (DeltaSeconds :type Float%20%28single-precision%29))
  (bind _charactermovement (Variables|Character|GetCharacterMovement))
  (bind _asmy_aicharacter (Utilities|Casting|CastToMyAICharacter (Class|PawnMovementComponent|GetPawnOwner _charactermovement)))
  (bind _output_get (Variables|Default|SetMyCharacter _asmy_aicharacter))
  (if (Variables|/Script/MothGame.MyAICharacter|GetisAlert _output_get)
    (bind _output_get_2 (Variables|Default|SetMoveSpeed 7e+02))
    (Variables|/Script/Engine.CharacterMovementComponent|SetMaxWalkSpeed _charactermovement _output_get_2)
    (else
      (Utilities|FlowControl|Delay 3.0)
      (AI|Navigation|SimpleMovetoLocation (Pawn|GetController (Variables|Default|GetMyCharacter)) (.RandomLocation (Class|NavigationSystemV1|GetRandomPointinNavigableRadius (Variables|/Script/MothGame.MyAICharacter|GetvecOPos (Variables|Default|GetMyCharacter)) (Variables|Default|GetRadius) 0 0)))
      (Utilities|FlowControl|Delay 3.0)
      (Development|PrintText "Hello"))))

(fn ConstructionScript)