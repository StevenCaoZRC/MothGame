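; Checkpoint trigger actor that saves the player's location or, when NotEndOfLevel is off, marks the end of a level.
; On any Box overlap, a normal checkpoint writes player 0's location and IsEndOfLevelSaved = true to a SavedCheckPoint slot, creating it if missing, then destroys itself.
; The end-of-level branch only sets that flag false in the loaded save, without creating one or destroying the actor.
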(event OnComponentBeginOverlap(Box)
  (params (OverlappedComponent :type Primitive%20Component%20Object%20Reference) (OtherActor :type Actor%20Object%20Reference) (OtherComp :type Primitive%20Component%20Object%20Reference) (OtherBodyIndex :type Integer) (bFromSweep :type Boolean) (SweepResult :type Hit%20Result%20Structure%20%28by%20ref%29))
  (bind _saveslotname (Variables|Default|GetSaveSlotName))
  (bind _saveslotname_2 (Variables|Default|GetSaveSlotName))
  (if (Variables|Default|GetNot%20End%20of%20Level)
    ;[0 0 0] Saving Player Location
    (Utilities|FlowControl|Sequence
      (:then_0
        (bind _asbp_moth_game_character (Utilities|Casting|CastToBP_MothGameCharacter (Game|GetPlayerCharacter 0)))
        (Variables|Default|SetPlayerLoc (Transformation|GetActorLocation _asbp_moth_game_character))
        (Development|PrintString "CheckPointReached"))
      (:then_1
        (bind _returnvalue (SaveGame|DoesSaveGameExist (Variables|Default|GetSaveSlotName)))
        (if _returnvalue
          (bind _returnvalue_2 (SaveGame|LoadGamefromSlot (Variables|Default|GetSaveSlotName)))
          (bind _assaved_check_point (Utilities|Casting|CastToSavedCheckPoint _returnvalue_2))
          (Variables|/Game/Checkpoint/SavedCheckPoint.SavedCheckPoint_C|SetSavedLoc _assaved_check_point (Variables|Default|GetPlayerLoc))
          (Variables|/Game/Checkpoint/SavedCheckPoint.SavedCheckPoint_C|SetIsEndOfLevelSaved _assaved_check_point true)
          (SaveGame|SaveGametoSlot _assaved_check_point _saveslotname)
          (else
            (bind _returnvalue_3 (SaveGame|CreateSaveGameObject "/Game/Checkpoint/SavedCheckPoint.SavedCheckPoint_C"))
            (Variables|/Game/Checkpoint/SavedCheckPoint.SavedCheckPoint_C|SetSavedLoc _returnvalue_3 (Variables|Default|GetPlayerLoc))
            (Variables|/Game/Checkpoint/SavedCheckPoint.SavedCheckPoint_C|SetIsEndOfLevelSaved _returnvalue_3 true)
            (SaveGame|SaveGametoSlot _returnvalue_3 _saveslotname)))
        (Actor|DestroyActor)))
    (else
      ;[0 0 0] Check if player reach the end of the level
      (bind _returnvalue_4 (SaveGame|LoadGamefromSlot _saveslotname_2))
      (bind _assaved_check_point_2 (Utilities|Casting|CastToSavedCheckPoint _returnvalue_4))
      (Variables|/Game/Checkpoint/SavedCheckPoint.SavedCheckPoint_C|SetIsEndOfLevelSaved _assaved_check_point_2 false)
      (SaveGame|SaveGametoSlot _assaved_check_point_2 _saveslotname_2))))

(event EventBeginPlay)

(event Collision|EventActorBeginOverlap
  (params (OtherActor :type Actor%20Object%20Reference)))

(event EventTick
  (params (DeltaSeconds :type Float%20%28single-precision%29)))

(fn ConstructionScript)