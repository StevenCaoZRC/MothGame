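; BP_Shard is a health pickup that bobs on a sine wave and grants the moth player timed health regeneration.
; Box overlap copies RegenRate to the character, hides the shard and sets StartRegen.
; Tick then loops through a one-second Delay, decrementing EffectDuration and calling the cached player's CallHPRegen and UpdateHealth until it hits zero and the shard destroys itself.
; Debug prints show start location and player health.
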(event OnComponentBeginOverlap(Box)
  (params (OverlappedComponent :type Primitive%20Component%20Object%20Reference) (OtherActor :type Actor%20Object%20Reference) (OtherComp :type Primitive%20Component%20Object%20Reference) (OtherBodyIndex :type Integer) (bFromSweep :type Boolean) (SweepResult :type Hit%20Result%20Structure%20%28by%20ref%29))
  (bind _asbp_moth_game_character (Utilities|Casting|CastToBP_MothGameCharacter OtherActor))
  (Variables|/Game/MothCharacter/BP_MothGameCharacter.BP_MothGameCharacter_C|SetRegenRate _asbp_moth_game_character (Variables|Default|GetRegenRate))
  (Variables|Default|SetStartRegen true)
  (Rendering|SetActorHiddenInGame true))

(event EventBeginPlay
  (bind _output_get (Variables|Default|SetStartLocation (Transformation|GetWorldLocation (Variables|Default|GetHealth_Shard))))
  (Development|PrintString (Utilities|String|ToString(Vector) _output_get))
  (Variables|Default|SetResetDuration (Variables|Default|GetEffectDuration))
  (bind _outactors (Actor|GetAllActorsOfClass "/Game/MothCharacter/BP_MothGameCharacter.BP_MothGameCharacter_C"))
  (Variables|Default|SetPlayer (Utilities|Array|Get(acopy) _outactors)))

(event Collision|EventActorBeginOverlap
  (params (OtherActor :type Actor%20Object%20Reference)))

(event EventTick
  (params (DeltaSeconds :type Float%20%28single-precision%29))
  (Development|PrintString (Utilities|String|ToString(Float) (Variables|/Script/MothGame.MothGameCharacter|GetCurrentHealth (Variables|Default|GetPlayer))))
  (Transformation|SetActorLocation (+ (Variables|Default|GetStartLocation) (* (Variables|Default|GetBob) (Math|Trig|Sin(Radians) (* (Utilities|Time|GetRealTimeSeconds) (Variables|Default|GetBobingSpeed))))) false false)
  (if (Variables|Default|GetStartRegen)
    (if (== (Variables|Default|GetEffectDuration) 0.0) :!label _label
      (Variables|Default|SetStartRegen false)
      (Actor|DestroyActor)
      (else
        (Utilities|FlowControl|Delay 1.0)
        (Variables|Default|SetEffectDuration (- (Variables|Default|GetEffectDuration) 1.0))
        (Default|CallHPRegen (Variables|Default|GetPlayer))
        (Default|UpdateHealth (Variables|Default|GetPlayer))
        (goto _label)))))

(fn ConstructionScript)