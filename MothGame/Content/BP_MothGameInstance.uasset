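; Game instance for the moth game that restores the player to a saved checkpoint and keeps that save only for the current session.
; SpawnFromSaved loads the SavedCheckPoint slot and, if its end-of-level flag is set, moves the player's moth character to the stored location.
; Shutdown deletes the save slot, so checkpoint progress does not persist after the game closes normally.
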(event Custom|SpawnFromSaved
  (bind _returnvalue (SaveGame|DoesSaveGameExist (Variables|Default|GetSaveNameSlot)))
  (if _returnvalue
    (bind _returnvalue_2 (SaveGame|LoadGamefromSlot (Variables|Default|GetSaveNameSlot)))
    (bind _assaved_check_point (Utilities|Casting|CastToSavedCheckPoint _returnvalue_2))
    (if (Variables|/Game/Checkpoint/SavedCheckPoint.SavedCheckPoint_C|GetIsEndOfLevelSaved _assaved_check_point)
      (bind _asbp_moth_game_character (Utilities|Casting|CastToBP_MothGameCharacter (Game|GetPlayerCharacter 0)))
      (Transformation|SetActorLocation _asbp_moth_game_character (Variables|/Game/Checkpoint/SavedCheckPoint.SavedCheckPoint_C|GetSavedLoc _assaved_check_point) false false))))

(event EventShutdown
  (SaveGame|DeleteGameinSlot (Variables|Default|GetSaveNameSlot)))